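; Player-controllable tank Blueprint that wires input to aiming and movement components.
; On BeginPlay it hands the barrel and turret to TankAiming and both tracks to TankMovement.
; Camera axes rotate an azimuth gimbal and spring arm, Fire calls TankAiming, and throttle axes feed TankMovement's forward and turn intents.
; The construction script assigns the track mesh and physical material to both tracks.
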(event EventBeginPlay
  (Class|TankAimingComponent|Initialise (Variables|Default|GetTankAiming) (Variables|Default|GetTankBarrel) (Variables|Default|GetTankTurret))
  (Class|TankMovementComponent|Initialise (Variables|Default|GetTankMovement) (Variables|Default|GetLeftTrack) (Variables|Default|GetRightTrack)))

(event Input|ActionEvents|InputActionFire
  (params (Key :type Key%20Structure :default "None"))
  ;[1 1 1] Fire Input BInding
  (:Pressed
    (Class|TankAimingComponent|Fire (Variables|Default|GetTankAiming))))

(event Input|AxisEvents|InputAxisAimAzimuth
  (params (AxisValue :type Float%20%28single-precision%29))
  ;[1 1 1] Camera Input Binding
  (Transformation|AddLocalRotation (Variables|Default|GetAzimuthGimbal) (Math|Rotator|MakeRotator 0.0 0.0 AxisValue) false false))

(event Input|AxisEvents|InputAxisAimElevation
  (params (AxisValue :type Float%20%28single-precision%29))
  ;[1 1 1] Camera Input Binding
  (Transformation|AddLocalRotation (Variables|Default|GetSpringArm) (Math|Rotator|MakeRotator 0.0 AxisValue 0.0) false false))

(event Input|AxisEvents|InputAxisMoveForward
  (params (AxisValue :type Float%20%28single-precision%29))
  ;[1 1 1] Throttle Input Binding
  (Class|TankMovementComponent|IntendMoveForward (Variables|Default|GetTankMovement) (+ AxisValue (* -1 (stale Input|AxisEvents|InputAxisMoveBackward AxisValue)))))

(event Input|AxisEvents|InputAxisMoveBackward
  (params (AxisValue :type Float%20%28single-precision%29))
  ;[1 1 1] Throttle Input Binding
)

(event Input|AxisEvents|InputAxisTurnRight
  (params (AxisValue :type Float%20%28single-precision%29))
  ;[1 1 1] Throttle Input Binding
  (Class|TankMovementComponent|IntendTurnRight (Variables|Default|GetTankMovement) (+ AxisValue (* -1 (stale Input|AxisEvents|InputAxisTurnLeft AxisValue)))))

(event Input|AxisEvents|InputAxisTurnLeft
  (params (AxisValue :type Float%20%28single-precision%29))
  ;[1 1 1] Throttle Input Binding
)

(fn ConstructionScript
  (bind _righttrack (Variables|Default|GetRightTrack))
  (bind _lefttrack (Variables|Default|GetLeftTrack))
  (Components|StaticMesh|SetStaticMesh _righttrack "/Game/Vehicles/SM_TankTrack.SM_TankTrack")
  (Class|PrimitiveComponent|SetPhysMaterialOverride _righttrack "/Game/Vehicles/M_Track.M_Track")
  (Components|StaticMesh|SetStaticMesh _lefttrack "/Game/Vehicles/SM_TankTrack.SM_TankTrack")
  (Class|PrimitiveComponent|SetPhysMaterialOverride _lefttrack "/Game/Vehicles/M_Track.M_Track"))